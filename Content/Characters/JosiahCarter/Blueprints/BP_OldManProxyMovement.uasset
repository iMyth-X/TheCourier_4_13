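; BP_OldManProxyMovement is a keyboard-driven proxy actor that moves and turns in the level, enabling player 0 input on BeginPlay.
; W/S and A/D translate it along its forward and right vectors, while Q/E yaw it, all at fixed delta-time-scaled rates.
; Each key press sets a flag and starts a zero-length RetriggerableDelay loop as a per-frame tick until release.
; Movement sets relative location from world location without sweeping, so it ignores collision.
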(event `self.ReceiveBeginPlay`
  (`self.EnableInput` (`GameplayStatics.GetPlayerController` 0)))

(event `Key|Q`
  (params (Key :type "Key Structure" :default "AnyKey"))
  ;[1 1 1] Rotate
  (:`Pressed`
    (set `self.isRotRight` true)
    (`KismetSystemLibrary.RetriggerableDelay` 0.0 :!label _label)
    (if (`self.isRotRight`)
      (`self.K2_AddActorLocalRotation` (`KismetMathLibrary.MakeRotator` 0.0 0.0 (* (`GameplayStatics.GetWorldDeltaSeconds`) -45.0)))
      (goto _label)))
  (:`Released`
    (set `self.isRotRight` false)))

(event `Key|E`
  (params (Key :type "Key Structure" :default "AnyKey"))
  ;[1 1 1] Rotate
  (:`Pressed`
    (set `self.isRotLeft` true)
    (`KismetSystemLibrary.RetriggerableDelay` 0.0 :!label _label_2)
    (if (`self.isRotLeft`)
      (`self.K2_AddActorLocalRotation` (`KismetMathLibrary.MakeRotator` 0.0 0.0 (* (`GameplayStatics.GetWorldDeltaSeconds`) 45.0)))
      (goto _label_2)))
  (:`Released`
    (set `self.isRotLeft` false)))

(event `Key|S`
  (params (Key :type "Key Structure" :default "AnyKey"))
  (:`Pressed`
    (set `self.isBackward` true)
    (`KismetSystemLibrary.RetriggerableDelay` 0.0 :!label _label_3)
    (if (`self.isBackward`)
      (`self.K2_SetActorRelativeLocation` (+ (`self.K2_GetActorLocation`) (* (`self.GetActorForwardVector`) (* (`GameplayStatics.GetWorldDeltaSeconds`) -45.0))))
      (goto _label_3)))
  (:`Released`
    (set `self.isBackward` false)))

(event `Key|W`
  (params (Key :type "Key Structure" :default "AnyKey"))
  (:`Pressed`
    (set `self.isForward` true)
    (`KismetSystemLibrary.RetriggerableDelay` 0.0 :!label _label_4)
    (if (`self.isForward`)
      (`self.K2_SetActorRelativeLocation` (+ (`self.K2_GetActorLocation`) (* (`self.GetActorForwardVector`) (* (`GameplayStatics.GetWorldDeltaSeconds`) 45.0))))
      (goto _label_4)))
  (:`Released`
    (set `self.isForward` false)))

(event `Key|D`
  (params (Key :type "Key Structure" :default "AnyKey"))
  (:`Pressed`
    (set `self.isRight` true)
    (`KismetSystemLibrary.RetriggerableDelay` 0.0 :!label _label_5)
    (if (`self.isRight`)
      (`self.K2_SetActorRelativeLocation` (+ (`self.K2_GetActorLocation`) (* (`self.GetActorRightVector`) (* (`GameplayStatics.GetWorldDeltaSeconds`) 45.0))))
      (goto _label_5)))
  (:`Released`
    (set `self.isRight` false)))

(event `Key|A`
  (params (Key :type "Key Structure" :default "AnyKey"))
  (:`Pressed`
    (set `self.isLeft` true)
    (`KismetSystemLibrary.RetriggerableDelay` 0.0 :!label _label_6)
    (if (`self.isLeft`)
      (`self.K2_SetActorRelativeLocation` (+ (`self.K2_GetActorLocation`) (* (`self.GetActorRightVector`) (* (`GameplayStatics.GetWorldDeltaSeconds`) -45.0))))
      (goto _label_6)))
  (:`Released`
    (set `self.isLeft` false)))

(fn `UserConstructionScript`)