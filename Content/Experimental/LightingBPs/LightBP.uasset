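; Pickupable candle light actor with three flame particles that go out when its material is transformed.
; The material transform component's events deactivate the flames on transform and reactivate them on untransform.
; Pickup, gated by Pickupable, disables candle physics and attaches the root to the given target; Drop re-enables physics and detaches.
; SetFlameAttributes randomises flicker and brightness and applies texture and color, but its construction-script calls are disconnected.
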(event `self.ReceiveBeginPlay`
  (bind _bp_materialtransformcomponent (`self.BP_MaterialTransformComponent`))
  (add `/Game/Environment/Interactable/LampOfAlhazred/Blueprints/BP_MaterialTransformComponent.OnMaterialTransform` _bp_materialtransformcomponent (delegate `OnMaterialTransform`))
  (add `/Game/Environment/Interactable/LampOfAlhazred/Blueprints/BP_MaterialTransformComponent.OnMaterialUntransform` _bp_materialtransformcomponent (delegate `OnMaterialUntransform`)))

(event `OnMaterialTransform`
  (`ActorComponent.Deactivate` (`self.Flame2`))
  (`ActorComponent.Deactivate` (`self.Flame1`))
  (`ActorComponent.Deactivate` (`self.Flame3`)))

(event `OnMaterialUntransform`
  (`ActorComponent.Activate` (`self.Flame1`) true)
  (`ActorComponent.Activate` (`self.Flame2`) true)
  (`ActorComponent.Activate` (`self.Flame3`) true))

(event `/Game/VirtualRealityBP/Blueprints/PickupActorInterface.Pickup`
  (params (AttachTo :type "SceneComponent Object Reference"))
  (if (`self.Pickupable`)
    (`PrimitiveComponent.SetSimulatePhysics` (`self.Candles`) false)
    (`SceneComponent.K2_AttachToComponent` (`self.K2_GetRootComponent`) AttachTo "None" "KeepWorld" "KeepWorld" "KeepWorld" false)))

(event `/Game/VirtualRealityBP/Blueprints/PickupActorInterface.Drop`
  (`PrimitiveComponent.SetSimulatePhysics` (`self.Candles`) true)
  (`self.K2_DetachFromActor` "KeepWorld" "KeepWorld" "KeepWorld"))

(fn `SetFlameAttributes`
  (params (FlameParticle :type "ParticleSystemComponent Object Reference"))
  (bind _returnvalue (`PrimitiveComponent.CreateDynamicMaterialInstance` FlameParticle 0 (`PrimitiveComponent.GetMaterial` FlameParticle 0)))
  (`MaterialInstanceDynamic.SetTextureParameterValue` _returnvalue "FlameImage" (`self.FlameTexture`))
  (`MaterialInstanceDynamic.SetScalarParameterValue` _returnvalue "FlickerSpeed" (`KismetMathLibrary.RandomFloatInRange` (`self.FlameSway_Min`) (`self.FlameSway_Max`)))
  (`MaterialInstanceDynamic.SetScalarParameterValue` _returnvalue "Emissive" (`self.FlameEmissiveStrength`))
  (`ParticleSystemComponent.SetColorParameter` FlameParticle "Color" (`self.Flamecolor`))
  (`ParticleSystemComponent.SetFloatParameter` FlameParticle "Brightness" (`KismetMathLibrary.RandomFloatInRange` (`self.Brightness_Min`) (`self.Brightness_Max`)))
  (`ParticleSystemComponent.SetFloatParameter` FlameParticle "Lifetime" (`KismetMathLibrary.RandomFloatInRange` (`self.Flicker_min`) (`self.Flicker_max`))))

(fn `UserConstructionScript`
  (`parent.UserConstructionScript`))