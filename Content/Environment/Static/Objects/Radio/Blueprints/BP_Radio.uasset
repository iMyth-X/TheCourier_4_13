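; BP_Radio is a radio prop that plays a tuning sound and blinks a point light, controlled by keyboard input enabled on BeginPlay.
; R starts the sound and an endless Delay-driven blink loop; T stops the sound and hides the light.
; T does not break the loop, so a running blink shows the light again.
; The IsOn and IsOff flags track key holds but are never read here.
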(event `self.ReceiveBeginPlay`
  (`self.EnableInput` (`GameplayStatics.GetPlayerController` 0)))

(event `Key|R`
  (params (Key :type "Key Structure" :default "AnyKey"))
  (:`Pressed`
    (set `self.isOn` true)
    (`self.RadioLightFlickerOn`))
  (:`Released`
    (set `self.isOn` false)))

(event `Key|T`
  (params (Key :type "Key Structure" :default "AnyKey"))
  (:`Pressed`
    (set `self.isOff` true)
    (`self.RadioLightFlickerOff`))
  (:`Released`
    (set `self.isOff` false)))

(event `RadioLightFlickerOn`
  (`AudioComponent.Play` (`self.Radio_Tuning_SFX`) 0.0)
  (`SceneComponent.SetVisibility` (`self.PointLight`) true false :!label _label)
  (`KismetSystemLibrary.Delay` 0.5)
  (`SceneComponent.SetVisibility` (`self.PointLight`) false false)
  (`KismetSystemLibrary.Delay` 1.0)
  (goto _label))

(event `RadioLightFlickerOff`
  (`AudioComponent.Stop` (`self.Radio_Tuning_SFX`))
  (`SceneComponent.SetVisibility` (`self.PointLight`) false false))

(fn `UserConstructionScript`
  (`parent.UserConstructionScript`))