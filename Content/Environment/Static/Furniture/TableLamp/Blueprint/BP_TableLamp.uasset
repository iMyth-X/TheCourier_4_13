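; BP_TableLamp is a table lamp prop with a hanging piece, which can be picked up and dropped.
; The construction script links the hanging piece to the lamp body through a physics constraint.
; Pickup, gated by a Pickupable flag, turns off lamp physics and attaches the root component to the supplied component.
; Drop re-enables physics and detaches the actor, keeping its world transform.
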(event `/Game/VirtualRealityBP/Blueprints/PickupActorInterface.Pickup`
  (params (AttachTo :type "SceneComponent Object Reference"))
  (if (`self.pickupable`)
    (`PrimitiveComponent.SetSimulatePhysics` (`self.TableLamp`) false)
    (`SceneComponent.K2_AttachToComponent` (`self.K2_GetRootComponent`) AttachTo "None" "KeepWorld" "KeepWorld" "KeepWorld" true)))

(event `self.ReceiveTick`
  (params (DeltaSeconds :type "Float (single-precision)")))

(event `/Game/VirtualRealityBP/Blueprints/PickupActorInterface.Drop`
  (`PrimitiveComponent.SetSimulatePhysics` (`self.TableLamp`) true)
  (`self.K2_DetachFromActor` "KeepWorld" "KeepWorld" "KeepWorld"))

(fn `UserConstructionScript`
  (`PhysicsConstraintComponent.SetConstrainedComponents` (`self.PhysicsConstraint`) (`self.HangingPiece`) "None" (`self.TableLamp`) "None"))