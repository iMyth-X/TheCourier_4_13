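; Test grandfather clock actor that animates four hands from an accumulated clock time with adjustable speed.
; Construction converts each hand's seconds per rotation into a roll rate.
; Tick scales delta time by SpeedOfTime, and SetClockTime sets each hand's roll from the total, printed on screen for debugging.
; Keys 1–3 switch the time multiplier; an incremental rotation variant, UpdateClockTime, exists but is not called here.
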(event `self.ReceiveTick`
  (params (DeltaSeconds :type "Float (single-precision)"))
  (`self.UpdateClock` DeltaSeconds)
  ;[1 1 1] Testing Purposes
  (`KismetSystemLibrary.PrintString` (`KismetStringLibrary.Conv_DoubleToString` (`self.TotalTime`)) true false (struct :`R` 0.095608 :`G` 0.137434 :`B` 1.0 :`A` 1.0) 0.01))

(event `self.ReceiveBeginPlay`
  ;[1 1 1] Testing Purposes
  (`self.EnableInput` (`GameplayStatics.GetPlayerController` 0)))

(event `Key|One`
  (params (Key :type "Key Structure" :default "AnyKey"))
  ;[1 1 1] Testing Purposes
  (:`Pressed`
    (set `self.SpeedOfTime` 1.0)))

(event `Key|Two`
  (params (Key :type "Key Structure" :default "AnyKey"))
  ;[1 1 1] Testing Purposes
  (:`Pressed`
    (set `self.SpeedOfTime` 2.0)))

(event `Key|Three`
  (params (Key :type "Key Structure" :default "AnyKey"))
  ;[1 1 1] Testing Purposes
  (:`Pressed`
    (set `self.SpeedOfTime` 3.0)))

(fn `SetClockTime`
  (params (TimeSinceStart :type "Float (double-precision)"))
  (for _index (range (`self.NumberOfHands`))
    (bind _item (`KismetArrayLibrary.Array_Get` (`self.HandList`) _index))
    (`SceneComponent.K2_SetRelativeRotation` _item (`KismetMathLibrary.MakeRotator` (* (`KismetArrayLibrary.Array_Get` (`self.HandRotateSpeedList`) _index) TimeSinceStart) (.pitch (`SceneComponent.RelativeRotation` _item)) (.yaw (`SceneComponent.RelativeRotation` _item))) false false)))

(fn `UpdateClock`
  (params (DeltaTime :type "Float (double-precision)"))
  (locals (NewDeltaTime :type "Float (double-precision)"))
  (bind _output_get (set `local.NewDeltaTime` (* DeltaTime (`self.SpeedOfTime`))))
  (bind _output_get_2 (set `self.TotalTime` (+ _output_get (`self.TotalTime`))))
  (`self.SetClockTime` _output_get_2))

(fn `UpdateClockTime`
  (params (DeltaTime :type "Float (double-precision)"))
  (for _index (range (`self.NumberOfHands`))
    (bind _item (`KismetArrayLibrary.Array_Get` (`self.HandList`) _index))
    (`SceneComponent.K2_SetRelativeRotation` _item (`KismetMathLibrary.MakeRotator` (+ (.roll (`SceneComponent.RelativeRotation` _item)) (* (`KismetArrayLibrary.Array_Get` (`self.HandRotateSpeedList`) _index) DeltaTime)) (.pitch (`SceneComponent.RelativeRotation` _item)) (.yaw (`SceneComponent.RelativeRotation` _item))) false false)))

(fn `UserConstructionScript`
  (set `self.HandList` (`|MakeArray` (`self.Hand1_Anchor`) (`self.Hand2_Anchor`) (`self.Hand3_Anchor`) (`self.Hand4_Anchor`)))
  (for _array_element (`self.HandSecondsPerRotationList`)
    (`KismetArrayLibrary.Array_Add` (`self.HandRotateSpeedList`) (/ -360.0 (`KismetMathLibrary.Conv_IntToDouble` _array_element)))))